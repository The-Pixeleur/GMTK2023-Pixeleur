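; Betting window actor that the player uses to bet on a knight.
; Tick checks player distance and camera aim at the Cube, toggling a custom-depth highlight, the use prompt widget and actor input.
; The Utiliser action copies the knight's name, portrait data, equipment and luck into the bet widget and displays it.
; If betting is unavailable, it shows a bottom-text refusal message instead.
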(event EventBeginPlay
  (bind _returnvalue (UserInterface|CreateWidget "/Game/UI/UI_Use.UI_Use_C"))
  (bind _output_get (Variables|Default|SetUI _returnvalue))
  (UserInterface|Viewport|AddtoViewport _output_get 0)
  (bind _returnvalue_2 (UserInterface|CreateWidget "/Game/UI/UI_bet.UI_bet_C"))
  (Variables|Default|SetUibet _returnvalue_2))

(event EventTick
  (params (DeltaSeconds :type Float%20%28single-precision%29))
  (bind _returnvalue (Game|GetPlayerController 0))
  (bind _returnvalue_2 (Game|GetPlayerCameraManager 0))
  (bind _cube (Variables|Default|GetCube))
  (bind _ui (Variables|Default|GetUI))
  (if (<= (Transformation|GetDistanceTo self (Game|GetPlayerCharacter 0)) 1.1e+02)
    (if (>= (Math|Vector|DotProduct (Transformation|GetActorForwardVector _returnvalue_2) (Math|Vector|GetUnitDirection(Vector) (Camera|GetCameraLocation _returnvalue_2) (Transformation|GetWorldLocation (Variables|Default|GetCube)))) 0.975)
      (Rendering|SetRenderCustomDepth _cube true)
      (if (not (Widget|IsVisible _ui))
        (UserInterface|Viewport|AddtoViewport _ui 0)
        (Input|EnableInput _returnvalue))
      (else
        (Rendering|SetRenderCustomDepth _cube false)
        (Widget|RemovefromParent _ui)
        (Input|DisableInput _returnvalue)))
    (else
      (Rendering|SetRenderCustomDepth _cube false)
      (Widget|RemovefromParent _ui)
      (Input|DisableInput (Game|GetPlayerController 0)))))

(event Input|ActionEvents|InputActionUtiliser
  (params (Key :type Key%20Structure :default "None"))
  (bind _uibet (Variables|Default|GetUibet))
  (:Pressed
    (if (Variables|Default|GetCanBet?)
      (Variables|/Game/UI/UI_bet.UI_bet_C|SetKnightName _uibet (Variables|Default|GetKnightName))
      (Variables|/Game/UI/UI_bet.UI_bet_C|SetKnightPP _uibet (Variables|Default|GetKnightPP))
      (Variables|/Game/UI/UI_bet.UI_bet_C|SetEquippedWith _uibet (Variables|Default|GetEquipped%20With))
      (Variables|/Game/UI/UI_bet.UI_bet_C|SetLuck _uibet (Variables|Default|GetKnightLuck))
      (UserInterface|Viewport|AddtoViewport _uibet 0)
      (else
        (bind _returnvalue (UserInterface|CreateWidget "/Game/UI/UI_texteBas.UI_texteBas_C"))
        (Variables|/Game/UI/UI_texteBas.UI_texteBas_C|SetText _returnvalue "I can't bet right now.")
        (UserInterface|Viewport|AddtoViewport _returnvalue 0)))))

(fn ConstructionScript)