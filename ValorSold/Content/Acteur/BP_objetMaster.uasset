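; Base interactable object actor that shows a use prompt when the first-person player is near and looking at it, and can be assigned as their inventory item.
; BeginPlay creates a UI_Use widget labeled from the SObject name and class.
; Tick checks distance and a camera dot product to toggle the widget, custom-depth highlight and input.
; The Utiliser action stores the object's class in the character's InventoryItem, leaving the actor in place.
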(event EventBeginPlay
  (bind _s_object (Variables|Default|GetS_object))
  (bind (_icon _name _sellprice _percenttowinmin _percenttowinmax _objectclass) (Utilities|Struct|BreakS_object _s_object))
  (bind _returnvalue (UserInterface|CreateWidget "/Game/UI/UI_Use.UI_Use_C"))
  (bind _output_get (Variables|Default|SetUI _returnvalue))
  (Variables|/Game/UI/UI_Use.UI_Use_C|SetText _output_get (Utilities|Text|ToText(String) (Utilities|String|Append (Utilities|String|ToString(Text) _name) " 
" "Class : \"" (Utilities|String|ToString(Text) _objectclass) "\"")))
  (UserInterface|Viewport|AddtoViewport _output_get 0))

(event Collision|EventActorBeginOverlap
  (params (OtherActor :type Actor%20Object%20Reference)))

(event EventTick
  (params (DeltaSeconds :type Float%20%28single-precision%29))
  (bind _returnvalue (Game|GetPlayerController 0))
  (bind _returnvalue_2 (Game|GetPlayerCameraManager 0))
  (bind _cube1 (Variables|Default|GetCube1))
  (bind _ui (Variables|Default|GetUI))
  (if (<= (Transformation|GetDistanceTo self (Game|GetPlayerCharacter 0)) 1.5e+02)
    (if (>= (Math|Vector|DotProduct (Transformation|GetActorForwardVector _returnvalue_2) (Math|Vector|GetUnitDirection(Vector) (Camera|GetCameraLocation _returnvalue_2) (Transformation|GetWorldLocation (Variables|Default|GetCube1)))) 0.975)
      (Rendering|SetRenderCustomDepth _cube1 true)
      (if (not (Widget|IsVisible _ui))
        (UserInterface|Viewport|AddtoViewport _ui 0)
        (Input|EnableInput _returnvalue))
      (else
        (Rendering|SetRenderCustomDepth _cube1 false)
        (Widget|RemovefromParent _ui)
        (Input|DisableInput _returnvalue)))
    (else
      (Rendering|SetRenderCustomDepth _cube1 false)
      (Widget|RemovefromParent _ui)
      (Input|DisableInput (Game|GetPlayerController 0)))))

(event Input|ActionEvents|InputActionUtiliser
  (params (Key :type Key%20Structure :default "None"))
  (:Pressed
    (bind _asbp_first_person_character (Utilities|Casting|CastToBP_FirstPersonCharacter (Game|Player|GetPlayerPawn 0)))
    (Variables|/Game/FirstPerson/Blueprints/BP_FirstPersonCharacter.BP_FirstPersonCharacter_C|SetInventoryItem _asbp_first_person_character (Utilities|GetClass self))))

(fn ConstructionScript)