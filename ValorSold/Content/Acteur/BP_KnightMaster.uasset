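; BP_KnightMaster is a knight NPC that opens a dialogue with the player and requests a random item.
; StartDialogue fills a UI_dialogue widget from the SKnight struct, turns the AI's focus to the player and switches input to mouse-driven UI.
; ItemWanted then picks a random entry from the wanted-item list, shows it in the widget and stores it as the player character's ItemToSell.
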(event Custom|StartDialogue
  (bind _returnvalue (Game|GetPlayerController 0))
  (bind _returnvalue_2 (Game|GetPlayerCharacter 0))
  (bind _s_knight (Variables|Default|GetS_knight))
  (bind (_knightprofilpic _name _welcomingtext) (Utilities|Struct|BreakS_Knight _s_knight))
  (bind _returnvalue_3 (UserInterface|CreateWidget "/Game/UI/UI_dialogue.UI_dialogue_C"))
  (Variables|/Game/UI/UI_dialogue.UI_dialogue_C|SetKnightPP _returnvalue_3 _knightprofilpic)
  (Variables|/Game/UI/UI_dialogue.UI_dialogue_C|SetName _returnvalue_3 _name)
  (Variables|/Game/UI/UI_dialogue.UI_dialogue_C|SetWelcomeText _returnvalue_3 _welcomingtext)
  (UserInterface|Viewport|AddtoViewport _returnvalue_3 0)
  (AI|SetFocus (AI|GetAIController self) _returnvalue_2)
  (Input|DisableInput _returnvalue_2 _returnvalue)
  (Input|SetInputModeUIOnly _returnvalue 0 "DoNotLock" false)
  (Variables|/Script/Engine.PlayerController|SetbShowMouseCursor _returnvalue true)
  (CallFunction|ItemWanted))

(event Custom|ItemWanted
  (bind _itemwantedliste (Variables|Default|GetItemwantedListe))
  (bind _output_get (Variables|Default|SetItemWantedRef (Utilities|Array|Get(acopy) _itemwantedliste (Math|Random|RandomIntegerinRange 0 (Utilities|Array|LastIndex _itemwantedliste)))))
  (bind _output_get_2 (Variables|/Game/UI/UI_dialogue.UI_dialogue_C|SetObjectWanted (stale Custom|StartDialogue _returnvalue_3) (Utilities|Text|ToText(Name) (Utilities|String|StringToName (Utilities|String|EnumtoString _output_get)))))
  (bind _asbp_first_person_character (Utilities|Casting|CastToBP_FirstPersonCharacter (Game|Player|GetPlayerPawn 0)))
  (Variables|/Game/FirstPerson/Blueprints/BP_FirstPersonCharacter.BP_FirstPersonCharacter_C|SetItemToSell _asbp_first_person_character (Utilities|String|ToString(Text) _output_get_2)))

(fn ConstructionScript)